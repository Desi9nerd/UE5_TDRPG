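; RPG player character Blueprint that adds debug hotkeys and a motion-warping hook for facing a target.
; Keys toggle pause, step briefly from pause via a near-zero timer, and cycle stat overlays through FlipFlop and MultiGate console commands.
; Shift+H switches the static mesh show flag through a non-looping MultiGate.
; UpdateFacingTarget feeds a location into the "FacingTarget" warp target, which montage MotionWarping notify states reference by name.
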(event `Key|P` :paused true
  (params (Key :type "Key Structure"))
  (:`Pressed`
    (if (`GameplayStatics.IsGamePaused`)
      (`GameplayStatics.SetGamePaused` false)
      (else
        (`GameplayStatics.SetGamePaused` true)))))

(event `Key|Shift+One`
  (params (Key :type "Key Structure"))
  (:`Pressed`
    (`/Engine/EditorBlueprintResources/StandardMacros.FlipFlop`
      (:`A`
        (`KismetSystemLibrary.ExecuteConsoleCommand` "stat fps \nstat unit \nt.maxfps 999" null))
      (:`B`
        (`KismetSystemLibrary.ExecuteConsoleCommand` "stat fps \nstat unit" null)))))

(event `Key|Shift+Two`
  (params (Key :type "Key Structure"))
  (:`Pressed`
    (`|MultiGate` false true
      (:`Out 0`
        (`KismetSystemLibrary.ExecuteConsoleCommand` "stat game" null))
      (:`Out 1`
        (`KismetSystemLibrary.ExecuteConsoleCommand` "stat game" null))
      (:`Out 2`
        (`KismetSystemLibrary.ExecuteConsoleCommand` "stat scenerendering" null))
      (:`Out 3`
        (`KismetSystemLibrary.ExecuteConsoleCommand` "stat scenerendering" null))
      (:`Out 4`
        (`KismetSystemLibrary.ExecuteConsoleCommand` "stat gpu" null))
      (:`Out 5`
        (`KismetSystemLibrary.ExecuteConsoleCommand` "stat gpu" null)))))

(event `Key|SpaceBar`
  (params (Key :type "Key Structure"))
  (:`Pressed`
    (if (`GameplayStatics.IsGamePaused`)
      (`GameplayStatics.SetGamePaused` false)
      (`KismetSystemLibrary.K2_SetTimerDelegate` (delegate `StepOnceAndPause`) 1e-06))))

(event `StepOnceAndPause`
  (`GameplayStatics.SetGamePaused` (not (`GameplayStatics.IsGamePaused`))))

(event `Key|Shift+H`
  (params (Key :type "Key Structure"))
  (:`Pressed`
    (`|MultiGate` false
      (:`Out 0`
        (bind _isa (`/Engine/EditorBlueprintResources/StandardMacros.FlipFlop` :!label _label)
          (:`A`
            _)
          (:`B`
            _))
        (`KismetSystemLibrary.ExecuteConsoleCommand` (`KismetStringLibrary.Concat_StrStr` "showflag:staticmeshes" (`KismetStringLibrary.Conv_IntToString` (`KismetMathLibrary.Conv_BoolToInt` (not _isa)))) null))
      (:`Out 1`
        (goto _label))
      (:`Out 2`
        (bind _isa_2 (`/Engine/EditorBlueprintResources/StandardMacros.FlipFlop` :!label _label_2)
          (:`A`
            _)
          (:`B`
            _))
        (`KismetSystemLibrary.ExecuteConsoleCommand` (`KismetStringLibrary.Concat_StrStr` "showflag:staticmeshes" (`KismetStringLibrary.Conv_IntToString` (`KismetMathLibrary.Conv_BoolToInt` (not _isa_2)))) null))
      (:`Out 3`
        (goto _label_2)))))

(event `self.UpdateFacingTarget`
  (params (Target :type "Vector Structure (by ref)"))
  (`MotionWarpingComponent.AddOrUpdateWarpTargetFromLocation` (`self.MotionWarpingComponent`) "FacingTarget" Target) ; 몽타주에서 MotionWarping 애님스테이트를 지정하고 Warp Target Name을 똑같이 적는다
)

(fn `UserConstructionScript`)