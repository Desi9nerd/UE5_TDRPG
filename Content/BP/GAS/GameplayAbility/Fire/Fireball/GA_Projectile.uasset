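; GA_Projectile is a gameplay ability that launches a fireball projectile toward the point under the mouse.
; On activation it takes target data under the mouse, turns the avatar toward that location through an interface message, and plays a cast montage.
; The Event.Montage.Fireball gameplay event from the montage triggers the projectile spawn at the stored location.
; The ability ends when the montage completes, blends out, or is interrupted or cancelled.
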(event `self.K2_ActivateAbility`
  (bind (_asynctaskproxy _datahandle) (`TDAT_TargetData.CreateTargetDataUnderMouse`)
    (:`ValidData`
      (set `self.ProjectileTargetLocation` (`.Location` (`GameplayStatics.BreakHitResult` (`AbilitySystemBlueprintLibrary.GetHitResultFromTargetData` _datahandle))))
      ;[1 1 1] Comment
      (message `ICombat.UpdateFacingTarget` (`self.GetAvatarActorFromActorInfo`) (`self.ProjectileTargetLocation`))
      (`AbilityTask_PlayMontageAndWait.CreatePlayMontageAndWaitProxy` "None" "/Game/ABP/Ryu/Montages/AM_Test.AM_Test"
        (:`then`
          (`AbilityTask_WaitGameplayEvent.WaitGameplayEvent` (struct :`TagName` "Event.Montage.Fireball") null
            (:`EventReceived`
              (`self.SpawnProjectile` (`self.ProjectileTargetLocation`)))))
        (:`OnCompleted`
          (`self.K2_EndAbility` :!label _label))
        (:`OnBlendOut`
          (goto _label))
        (:`OnInterrupted`
          (goto _label))
        (:`OnCancelled`
          (goto _label))))))