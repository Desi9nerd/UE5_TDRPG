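; Enemy Gameplay Ability for a ranged projectile attack, currently inert in this graph because ActivateAbility is empty and the attack chain is disconnected.
; The unwired chain turns the avatar toward its combat target, plays a random tagged attack montage and waits for that montage's gameplay event.
; On that event it calls SpawnProjectile at the target's current location, leaving the fetched socket location unused.
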(event `self.K2_ActivateAbility`)