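; Gameplay Ability for an enemy ranged attack that fires a projectile at the avatar's combat target.
; On activation it updates the avatar's facing toward the target and plays a random tagged attack montage.
; The montage's gameplay event triggers SpawnProjectile from the tagged socket at the target's current location, with an optional pitch override.
; The event wait triggers only once to prevent duplicate spawns.
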(event `self.K2_ActivateAbility`
  (bind _returnvalue (`self.GetAvatarActorFromActorInfo`))
  (bind _returnvalue_2 (message `ICombat.GetCombatTarget` _returnvalue))
  (message `ICombat.UpdateFacingTarget` _returnvalue (`Actor.K2_GetActorLocation` _returnvalue_2))
  (bind _returnvalue_3 (message `ICombat.GetAttackMontages` (`self.GetAvatarActorFromActorInfo`)))
  (bind _output_get (set `self.TaggedMontage` (`self.GetRandomTaggedMontageFromArray` _returnvalue_3)))
  (bind (_montage _montagetag _sockettag) (break `TaggedMontage` _output_get))
  (`AbilityTask_PlayMontageAndWait.CreatePlayMontageAndWaitProxy` "None" _montage 1.0 "None" false
    (:`then`
      (`AbilityTask_WaitGameplayEvent.WaitGameplayEvent` _montagetag null true ; Only Trigger Once를 체크하여 중복으로 스폰되는 것을 막음.
        (:`EventReceived`
          (bind _returnvalue_4 (message `ICombat.GetCombatTarget` (`self.GetAvatarActorFromActorInfo`)))
          (`self.SpawnProjectile` (`Actor.K2_GetActorLocation` _returnvalue_4) _sockettag (`self.ShouldOverridePitch`) 25.0))))))