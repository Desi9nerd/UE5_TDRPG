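; Enemy melee attack ability that turns the avatar toward its combat target and plays a random tagged montage.
; The montage's gameplay event triggers a radius search at the tagged combat socket for live players.
; Non-team hits receive the damage effect and blood effect, with debug drawing left in.
; Any hit fires one MeleeImpact cue tagged by montage; the ability then ends without stopping the montage.
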(event `self.K2_ActivateAbility`
  (bind _returnvalue (`self.GetAvatarActorFromActorInfo`))
  (bind _returnvalue_2 (`self.GetAvatarActorFromActorInfo`))
  (set `self.HasHitTarget` false)
  (bind _returnvalue_3 (message `ICombat.GetCombatTarget` _returnvalue_2))
  (bind _asicombat (cast `ICombat` _returnvalue_2))
  (`ICombat.UpdateFacingTarget` _asicombat (`Actor.K2_GetActorLocation` _returnvalue_3))
  ;[1 1 1] 캐릭터(BP_RPGCharacter / BP_Lich, Warrior)의 몽타주+Tag 가져오기
  (bind _returnvalue_4 (message `ICombat.GetAttackMontages` (`self.GetAvatarActorFromActorInfo`)))
  (bind _output_get (set `self.TaggedMontage` (`self.GetRandomTaggedMontageFromArray` _returnvalue_4)))
  (bind (_montage _montagetag _sockettag) (break `TaggedMontage` _output_get))
  (`AbilityTask_PlayMontageAndWait.CreatePlayMontageAndWaitProxy` "None" _montage 1.0 "None" false
    (:`then`
      (`AbilityTask_WaitGameplayEvent.WaitGameplayEvent` _montagetag null
        (:`EventReceived`
          (bind _returnvalue_5 (message `ICombat.GetCombatSocketLocation` _returnvalue _sockettag))
          (set `self.CombatSocketLocation` _returnvalue_5)
          (bind _outoverlappingactors (`TDAbilitySystemBPLibrary.GetLivePlayersWithinRadius` _returnvalue (`|MakeArray` _returnvalue) 40.0 (`self.CombatSocketLocation`)))
          (for _array_element _outoverlappingactors
            (if (not (`TDAbilitySystemBPLibrary.IsSameTeam` (`self.GetAvatarActorFromActorInfo`) _array_element))
              (`KismetSystemLibrary.DrawDebugSphere` (`Actor.K2_GetActorLocation` _array_element) 40.0 12 (struct :`R` 1.0 :`G` 0.290155 :`A` 1.0) 2.0)
              (`KismetSystemLibrary.PrintString` (`KismetSystemLibrary.GetObjectName` _array_element))
              (`TDAbilitySystemBPLibrary.ApplyDamageEffect` (`self.SetDamageEffectParams` _array_element))
              (set `self.HasHitTarget` true)
              (message `ICombat.GetBloodEffect` _array_element)))
          (if (`self.HasHitTarget`)
            (bind _returnvalue_6 (message `ICombat.GetCombatTarget` (`self.GetAvatarActorFromActorInfo`)))
            (`self.K2_ExecuteGameplayCueWithParams` (struct :`TagName` "GameplayCue.MeleeImpact") (`AbilitySystemBlueprintLibrary.MakeGameplayCueParameters` 0.0 0.0 (struct) (struct) (struct) (`BlueprintGameplayTagLibrary.MakeGameplayTagContainerFromTag` (`.MontageTag` (break `TaggedMontage` (`self.TaggedMontage`)))) (struct) (`self.CombatSocketLocation`) (0.0 0.0 0.0) null (`self.GetAvatarActorFromActorInfo`) _returnvalue_6)))
          (`self.K2_EndAbility`))))
    (:`OnCompleted`
      (`self.K2_EndAbility` :!label _label))
    (:`OnInterrupted`
      (goto _label))
    (:`OnCancelled`
      (goto _label))))