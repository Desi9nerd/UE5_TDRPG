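; Player gameplay ability that runs a four-stage, input-chained damage combo from sections of one montage, after checking cost and cooldown.
; A shared PlayMontageAndWait graph plays each section, waits for the montage's gameplay event and calls ApplyDamage at that hand's socket.
; ApplyDamage hits non-team players within a small radius with damage, knockback and blood effects; the projectile spawn is disconnected.
; Each hit before the last opens the next press; the final hit or a completed montage ends the ability.
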(event `self.K2_ActivateAbility`
  (bind _returnvalue (`self.K2_CheckAbilityCost`))
  (if _returnvalue
    (bind _returnvalue_2 (`self.K2_CheckAbilityCooldown`))
    (if _returnvalue_2
      (`self.K2_CommitAbility`)
      (`self.PlayMontageAndWait` "Combo1" (`self.SocketTag_Righthand`)
        (:`EventReceived`
          (`AbilityTask_WaitInputPress.WaitInputPress` false
            (:`OnPress`
              (`self.PlayMontageAndWait` "Combo2" (`self.SocketTag_Righthand`)
                (:`EventReceived`
                  (`AbilityTask_WaitInputPress.WaitInputPress` false
                    (:`OnPress`
                      (`self.PlayMontageAndWait` "Combo3" (`self.SocketTag_Righthand`)
                        (:`EventReceived`
                          (`AbilityTask_WaitInputPress.WaitInputPress` false
                            (:`OnPress`
                              (`self.PlayMontageAndWait` "Combo4" (`self.SocketTag_LeftHand`)
                                (:`EventReceived`
                                  (`self.K2_EndAbility`)))))))))))))))
      (else
        (`self.K2_EndAbility` :!label _label)))
    (else
      (goto _label))))

(fn `ApplyDamage`
  (params (CombatSocketTag :type "GameplayTag Structure (by ref)"))
  (bind _returnvalue (`self.GetAvatarActorFromActorInfo`))
  (bind _returnvalue_2 (message `ICombat.GetCombatSocketLocation` _returnvalue CombatSocketTag))
  (set `self.CombatSocketLocation` _returnvalue_2)
  (bind _outoverlappingactors (`TDAbilitySystemBPLibrary.GetLivePlayersWithinRadius` _returnvalue (`|MakeArray` _returnvalue) 150.0 (`self.CombatSocketLocation`)))
  (for _array_element _outoverlappingactors
    (if (not (`TDAbilitySystemBPLibrary.IsSameTeam` (`self.GetAvatarActorFromActorInfo`) _array_element))
      (`TDAbilitySystemBPLibrary.ApplyDamageEffect` (`self.SetDamageEffectParams` _array_element (`Actor.K2_GetActorLocation` (`self.GetAvatarActorFromActorInfo`)) true (1000.0 1000.0 1000.0) false (0.0 0.0 0.0) true 45.0))
      (message `ICombat.GetBloodEffect` _array_element))))