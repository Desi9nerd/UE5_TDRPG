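; GA_Combo is a player gameplay ability that runs a four-stage melee and projectile combo, advancing on input presses.
; A PlayMontageAndWait macro plays each montage section and waits for the ComboFlameShooting event, then applies damage and fires a projectile forward from the hand socket.
; ApplyDamage hits non-team players near that socket, triggering blood effects and debug output.
; The ability ends on montage completion or after the fourth hit; an older inline chain remains unconnected.
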(event `self.K2_ActivateAbility`
  (`self.PlayMontageAndWait` "Combo1" (`self.SocketTag_Righthand`)
    (:`EventReceived`
      (`AbilityTask_WaitInputPress.WaitInputPress` false
        (:`OnPress`
          (`self.PlayMontageAndWait` "Combo2" (`self.SocketTag_Righthand`)
            (:`EventReceived`
              (`AbilityTask_WaitInputPress.WaitInputPress` false
                (:`OnPress`
                  (`self.PlayMontageAndWait` "Combo3" (`self.SocketTag_Righthand`)
                    (:`EventReceived`
                      (`AbilityTask_WaitInputPress.WaitInputPress` false
                        (:`OnPress`
                          (`self.PlayMontageAndWait` "Combo4" (`self.SocketTag_LeftHand`)
                            (:`EventReceived`
                              (`self.K2_EndAbility`))))))))))))))))

(fn `ApplyDamage`
  (params (CombatSocketTag :type "GameplayTag Structure (by ref)"))
  (bind _returnvalue (`self.GetAvatarActorFromActorInfo`))
  (bind _returnvalue_2 (message `ICombat.GetCombatSocketLocation` _returnvalue CombatSocketTag))
  (set `self.CombatSocketLocation` _returnvalue_2)
  (bind _outoverlappingactors (`TDAbilitySystemBPLibrary.GetLivePlayersWithinRadius` _returnvalue (`|MakeArray` _returnvalue) 40.0 (`self.CombatSocketLocation`)))
  (for _array_element _outoverlappingactors
    (if (not (`TDAbilitySystemBPLibrary.IsSameTeam` (`self.GetAvatarActorFromActorInfo`) _array_element))
      (`KismetSystemLibrary.DrawDebugSphere` (`Actor.K2_GetActorLocation` _array_element) 40.0 12 (struct :`R` 1.0 :`G` 0.290155 :`A` 1.0) 2.0)
      (`KismetSystemLibrary.PrintString` (`KismetSystemLibrary.GetObjectName` _array_element))
      (`TDAbilitySystemBPLibrary.ApplyDamageEffect` (`self.SetDamageEffectParams` _array_element))
      (message `ICombat.GetBloodEffect` _array_element))))