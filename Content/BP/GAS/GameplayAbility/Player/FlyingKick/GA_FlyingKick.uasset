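; Gameplay Ability for the player's flying kick, which plays a kick montage and launches a projectile from the right leg.
; After cost and cooldown checks pass, it commits, plays the montage and waits once for the FlyingKick montage event.
; That event spawns the projectile at the right-leg socket, targeting a point horizontally ahead of the avatar.
; The ability ends on failed checks or any montage exit, while the montage may keep playing.
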(event `self.K2_ActivateAbility`
  (bind _returnvalue (`self.GetAvatarActorFromActorInfo`))
  (bind _returnvalue_2 (`self.K2_CheckAbilityCost`))
  (if _returnvalue_2
    (bind _returnvalue_3 (`self.K2_CheckAbilityCooldown`))
    (if _returnvalue_3
      (`self.K2_CommitAbility`)
      (`AbilityTask_PlayMontageAndWait.CreatePlayMontageAndWaitProxy` "None" "/Game/ABP/Ryu/Montages/Kick/AM_RYU_Kick.AM_RYU_Kick" 1.0 "None" false ; Stop when Ability Ends를 체크해제하면 Ability를 벗어나도 몽타주가 끝날 때까지 재생한다. 단 다른 몽타주 명령이 들어오면 끝긴다.
        (:`then`
          (`AbilityTask_WaitGameplayEvent.WaitGameplayEvent` (struct :`TagName` "Event.Montage.FlyingKick") null true
            (:`EventReceived`
              (`self.SpawnProjectile` (+ (`Actor.K2_GetActorLocation` _returnvalue) (* (`Actor.GetActorForwardVector` _returnvalue) (500.0 500.0 0.0))) (`self.RightLegSocketTag`)))))
        (:`OnCompleted`
          (`self.K2_EndAbility` :!label _label))
        (:`OnBlendOut`
          (goto _label))
        (:`OnInterrupted`
          (goto _label))
        (:`OnCancelled`
          (goto _label)))
      (else
        (`self.K2_EndAbility` :!label _label_2)))
    (else
      (goto _label_2))))