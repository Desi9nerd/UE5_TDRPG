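; Player gameplay ability that fires damaging magic arrow projectiles toward the point under the mouse.
; On activation it commits, gets the cursor hit, and tells the avatar to face that location while the magic arrow montage plays.
; A montage gameplay event spawns projectiles from the weapon socket with a pitch override, passing the hit actor as homing target.
; The montage may outlast the ability, which ends when the montage completes, blends out or is interrupted.
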(event `self.K2_ActivateAbility`
  (`self.K2_CommitAbility`)
  (bind (_asynctaskproxy _datahandle) (`TDAT_TargetData.CreateTargetDataUnderMouse`)
    (:`ValidData`
      (bind (_bblockinghit _binitialoverlap _time _distance _location _impactpoint _normal _impactnormal _physmat _hitactor) (`GameplayStatics.BreakHitResult` (`AbilitySystemBlueprintLibrary.GetHitResultFromTargetData` _datahandle)))
      (set `self.ProjectileTargetLocation` _location)
      (set `self.HitActor` _hitactor)
      (message `ICombat.UpdateFacingTarget` (`self.GetAvatarActorFromActorInfo`) (`self.ProjectileTargetLocation`))
      (`AbilityTask_PlayMontageAndWait.CreatePlayMontageAndWaitProxy` "None" "/Game/ABP/Ryu/Montages/AM_RYU_MagicArrow.AM_RYU_MagicArrow" 1.0 "None" false ; Stop when Ability Ends를 체크해제하면 Ability를 벗어나도 몽타주가 끝날 때까지 재생한다. 단 다른 몽타주 명령이 들어오면 끝긴다.
        (:`then`
          (`AbilityTask_WaitGameplayEvent.WaitGameplayEvent` (struct :`TagName` "Event.Montage.MagicArrow") null
            (:`EventReceived`
              (`self.SpawnProjectiles` (`self.ProjectileTargetLocation`) (`BlueprintGameplayTagLibrary.MakeLiteralGameplayTag` (struct :`TagName` "Socket.Weapon")) true 30.0 (`self.HitActor`)))))
        (:`OnCompleted`
          (`self.K2_EndAbility` :!label _label))
        (:`OnBlendOut`
          (goto _label))
        (:`OnInterrupted`
          (goto _label))
        (:`OnCancelled`
          (goto _label))))))